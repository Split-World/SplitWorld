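; Game mode for a split-world setup that gives the first player and any other players different spawn points.
; Its ChoosePlayerStart override records each player in a Players array, then searches all PlayerStart actors.
; A player whose object name contains "0" gets a start tagged Player1, while others get the first start without that tag.
; The event graph and construction script are empty.
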(event `self.ReceiveBeginPlay`)

(fn `ChoosePlayerStart`
  (params (Player :type "Controller Object Reference"))
  (returns (ReturnValue :type "Actor Object Reference"))
  (`KismetArrayLibrary.Array_Add` (`self.Players`) Player)
  (bind _outactors (`GameplayStatics.GetAllActorsOfClass` "/Script/Engine.PlayerStart"))
  (for _array_element _outactors
    (if (`KismetStringLibrary.Contains` (`KismetSystemLibrary.GetObjectName` Player) "0")
      (bind _returnvalue (`self.ActorHasTag` _array_element "Player1"))
      (if _returnvalue
        (return _array_element))
      (elif (not _returnvalue)
        (return _array_element)))))

(fn `UserConstructionScript`)