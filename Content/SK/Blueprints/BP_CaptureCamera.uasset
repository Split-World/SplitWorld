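; BP_CaptureCamera drives the clip plane of a masking scene capture between two players in a split-world setup.
; Tick resolves players from BP_SplitWorldGameMode, pairing one pawn with the other's Clone according to CameraIdx.
; For camera index 0 only, it places the plane at their midpoint, with the normal pointing from Player1 toward Player2.
; At short horizontal separation, the normal is flattened to 2D.
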(event `self.ReceiveTick`
  (params (DeltaSeconds :type "Float (single-precision)"))
  (bind _returnvalue (`self.K2_GetActorLocation` (`self.Player2`)))
  (bind _capturecomponent2d (`SceneCapture2D.CaptureComponent2D` (`self.Mask`)))
  (bind _returnvalue_2 (- (`self.K2_GetActorLocation` (`self.Player1`)) _returnvalue))
  (if (and (`KismetSystemLibrary.IsValid` (`self.Player1`)) (`KismetSystemLibrary.IsValid` (`self.Player2`)))
    (if (== (`self.CameraIdx`) 0)
      (set `SceneCaptureComponent2D.ClipPlaneBase` (+ (/ _returnvalue_2 2.0) _returnvalue) _capturecomponent2d)
      (if (< (`KismetMathLibrary.VSizeXY` _returnvalue_2) 300.0)
        (set `SceneCaptureComponent2D.ClipPlaneNormal` (* (`KismetMathLibrary.Vector_Normal2D` _returnvalue_2) -1.0) _capturecomponent2d)
        (else
          (set `SceneCaptureComponent2D.ClipPlaneNormal` (* (`KismetMathLibrary.Normal` _returnvalue_2) -1.0) _capturecomponent2d))))
    (else
      (bind _asbp_split_world_game_mode (cast `/Game/SK/Blueprints/BP_SplitWorldGameMode` (`GameplayStatics.GetGameMode`)))
      (bind _players (`/Game/SK/Blueprints/BP_SplitWorldGameMode.Players` _asbp_split_world_game_mode))
      (if (== (`KismetArrayLibrary.Array_Length` _players) 2)
        (bind _asbp_temp_player (cast `/Game/SK/Blueprints/BP_TempPlayer` (`Controller.K2_GetPawn` (`|GetArrayItem` _players))))
        (bind _asbp_temp_player_2 (cast `/Game/SK/Blueprints/BP_TempPlayer` (`Controller.K2_GetPawn` (`|GetArrayItem` _players 1))))
        (if (and (`KismetSystemLibrary.IsValid` (`/Game/SK/Blueprints/BP_TempPlayer.Clone` _asbp_temp_player)) (`KismetSystemLibrary.IsValid` (`/Game/SK/Blueprints/BP_TempPlayer.Clone` _asbp_temp_player_2)))
          (if (== (`self.CameraIdx`) 0)
            (set `self.Player1` _asbp_temp_player)
            (set `self.Player2` (`/Game/SK/Blueprints/BP_TempPlayer.Clone` _asbp_temp_player_2))
            (else
              (set `self.Player2` _asbp_temp_player_2)
              (set `self.Player1` (`/Game/SK/Blueprints/BP_TempPlayer.Clone` _asbp_temp_player)))))))))

(fn `UserConstructionScript`)